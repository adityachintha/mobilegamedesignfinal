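; BP_Hieroglyph is a collectible that awards points to the VR player when its static mesh is hit.
; On hit it plays a coin splash sound at the impact, prints a message, destroys itself, then adds 50 points to VRPawn.
; BeginPlay adds a rotating movement component for visual spin.
; An unconnected branch that would award points to BP_FirstPersonCharacter never runs.
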(event `self.StaticMesh.OnComponentHit`
  (params (HitComponent :type "PrimitiveComponent Object Reference") (OtherActor :type "Actor Object Reference") (OtherComp :type "PrimitiveComponent Object Reference") (NormalImpulse :type "Vector Structure") (Hit :type "HitResult Structure (by ref)"))
  ;[1 0.2467 0.162] Play Sound, Print and destroy on HIT
  (`GameplayStatics.PlaySoundAtLocation` "/Game/ChintaContent/Audio/coinsplash.coinsplash" (`.Location` (`GameplayStatics.BreakHitResult` Hit)) (struct) 1.0 1.0 0.0 null null null null)
  (`KismetSystemLibrary.PrintString` (`self.Message`))
  (`self.K2_DestroyActor`)
  ;[1 1 1] Gets points to VR Pawn
  (bind _asvrpawn (cast `/Game/VRTemplate/Blueprints/VRPawn` (`GameplayStatics.GetPlayerPawn` 0)))
  (`/Game/VRTemplate/Blueprints/VRPawn.AddVRPoints` _asvrpawn 50))

(event `self.ReceiveBeginPlay`
  ;[1 1 1] Rotating Visual
  (`AddComponent|NODE_AddRotatingMovementComponent-0`))

(fn `UserConstructionScript`)